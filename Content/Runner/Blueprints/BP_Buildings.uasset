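; Runner building segment that randomizes its scenery and triggers extension of the building chain.
; The construction script runs SpawnBuildings, which adds a child actor at each of six arrow markers through a separate random four-way pick.
; Any overlap with its Box calls ExtendBuilding on BP_RunnerGameMode, without filtering the overlapping actor.
; GetAttachPoint exposes the world transform of a separate Arrow as the segment's attach point.
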(event OnComponentBeginOverlap(Box)
  (params (OverlappedComponent :type Primitive%20Component%20Object%20Reference) (OtherActor :type Actor%20Object%20Reference) (OtherComp :type Primitive%20Component%20Object%20Reference) (OtherBodyIndex :type Integer) (bFromSweep :type Boolean) (SweepResult :type Hit%20Result%20Structure%20%28by%20ref%29))
  (bind _asbp_runner_game_mode (Utilities|Casting|CastToBP_RunnerGameMode (Game|GetGameMode)))
  (Default|ExtendBuilding _asbp_runner_game_mode))

(event EventBeginPlay)

(event Collision|EventActorBeginOverlap
  (params (OtherActor :type Actor%20Object%20Reference)))

(event EventTick
  (params (DeltaSeconds :type Float%20%28single-precision%29)))

(fn ConstructionScript
  (CallFunction|SpawnBuildings))

(fn GetAttachPoint
  (return (Transformation|GetWorldTransform (Variables|Default|GetArrow))))

(fn SpawnBuildings
  (bind _arrow4 (Variables|Default|GetArrow4))
  (bind _arrow5 (Variables|Default|GetArrow5))
  (bind _arrow6 (Variables|Default|GetArrow6))
  (bind _arrow1 (Variables|Default|GetArrow1))
  (bind _arrow2 (Variables|Default|GetArrow2))
  (bind _arrow3 (Variables|Default|GetArrow3))
  (bind _returnvalue (Transformation|GetRelativeTransform _arrow6))
  (bind _returnvalue_2 (Transformation|GetRelativeTransform _arrow3))
  (bind _returnvalue_3 (Transformation|GetRelativeTransform _arrow5))
  (bind _returnvalue_4 (Transformation|GetRelativeTransform _arrow4))
  (bind _returnvalue_5 (Transformation|GetRelativeTransform _arrow1))
  (bind _returnvalue_6 (Transformation|GetRelativeTransform _arrow2))
  (Utilities|FlowControl|Sequence
    (:then_0
      (switch int (Math|Random|RandomIntegerinRange 0 3)
        (:0
          (AddComponent|AddChildActorComponent false _returnvalue_5))
        (:1
          (AddComponent|AddChildActorComponent false _returnvalue_5))
        (:2
          (AddComponent|AddChildActorComponent false _returnvalue_5))
        (:3
          (AddComponent|AddChildActorComponent false _returnvalue_5))))
    (:then_1
      (switch int (Math|Random|RandomIntegerinRange 0 3)
        (:0
          (AddComponent|AddChildActorComponent false _returnvalue_6))
        (:1
          (AddComponent|AddChildActorComponent false _returnvalue_6))
        (:2
          (AddComponent|AddChildActorComponent false _returnvalue_6))
        (:3
          (AddComponent|AddChildActorComponent false _returnvalue_6))))
    (:then_2
      (switch int (Math|Random|RandomIntegerinRange 0 3)
        (:0
          (AddComponent|AddChildActorComponent false _returnvalue_2))
        (:1
          (AddComponent|AddChildActorComponent false _returnvalue_2))
        (:2
          (AddComponent|AddChildActorComponent false _returnvalue_2))
        (:3
          (AddComponent|AddChildActorComponent false _returnvalue_2))))
    (:then_3
      (switch int (Math|Random|RandomIntegerinRange 0 3)
        (:0
          (AddComponent|AddChildActorComponent false _returnvalue))
        (:1
          (AddComponent|AddChildActorComponent false _returnvalue))
        (:2
          (AddComponent|AddChildActorComponent false _returnvalue))
        (:3
          (AddComponent|AddChildActorComponent false _returnvalue))))
    (:then_4
      (switch int (Math|Random|RandomIntegerinRange 0 3)
        (:0
          (AddComponent|AddChildActorComponent false _returnvalue_3))
        (:1
          (AddComponent|AddChildActorComponent false _returnvalue_3))
        (:2
          (AddComponent|AddChildActorComponent false _returnvalue_3))
        (:3
          (AddComponent|AddChildActorComponent false _returnvalue_3))))
    (:then_5
      (switch int (Math|Random|RandomIntegerinRange 0 3)
        (:0
          (AddComponent|AddChildActorComponent false _returnvalue_4))
        (:1
          (AddComponent|AddChildActorComponent false _returnvalue_4))
        (:2
          (AddComponent|AddChildActorComponent false _returnvalue_4))
        (:3
          (AddComponent|AddChildActorComponent false _returnvalue_4))))))