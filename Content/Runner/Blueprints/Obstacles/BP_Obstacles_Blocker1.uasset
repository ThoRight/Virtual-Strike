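; BP_Obstacles_Blocker1 is a runner obstacle that kills the player on overlap unless they slide beneath it.
; On actor overlap it casts to BP_RunnerCharacter and spares a sliding character only when its own static mesh sits above a fixed world height.
; Otherwise it calls Death, plays a hit sound, and pauses the game after a short delay.
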(event Collision|EventActorBeginOverlap
  (params (OtherActor :type Actor%20Object%20Reference))
  (bind _asbp_runner_character (Utilities|Casting|CastToBP_RunnerCharacter OtherActor))
  (if (Variables|/Game/Runner/Blueprints/BP_RunnerCharacter.BP_RunnerCharacter_C|GetisSliding _asbp_runner_character)
    (if (not (> (.Z (Math|Vector|BreakVector (Transformation|GetWorldLocation (Variables|Default|GetStaticMesh)))) 9e+01))
      (Default|Death _asbp_runner_character :!label _label)
      (Audio|PlaySound2D "/Game/Runner/Something-being-hit-Sound-Effect.Something-being-hit-Sound-Effect" 1.0 1.0 0.0 0 0)
      (Utilities|FlowControl|Delay 1.0)
      (Game|SetGamePaused true))
    (else
      (goto _label))))

(fn ConstructionScript
  (|CallParentFunction))