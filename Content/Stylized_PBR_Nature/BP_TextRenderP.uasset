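; Text render actor, judging by its name, that follows player character 0 at a fixed, very low world height.
; Each tick it moves 400 units along the character's forward vector from their XY position, with Z pinned at -15000.
; It copies the character's roll and pitch and remaps yaw by sign: 180 plus yaw when negative, otherwise 360 minus yaw.
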(event EventTick
  (params (DeltaSeconds :type Float%20%28single-precision%29))
  (bind _returnvalue (Game|GetPlayerCharacter 0))
  (bind _returnvalue_2 (Game|GetPlayerCharacter 0))
  (bind _returnvalue_3 (Transformation|GetActorLocation _returnvalue))
  (bind _returnvalue_4 (Transformation|GetActorForwardVector _returnvalue))
  (bind _returnvalue_5 (Transformation|GetActorRotation _returnvalue_2))
  (bind _returnvalue_6 (* _returnvalue_4 "400.000000,400.000000,400.000000"))
  (bind _returnvalue_7 (+ _returnvalue_6 (Math|Vector|MakeVector (.x _returnvalue_3) (.y _returnvalue_3) 0.0)))
  (Transformation|SetActorLocation (Math|Vector|MakeVector (.x _returnvalue_7) (.y _returnvalue_7) -1.5e+04) false false)
  (if (< (.yaw _returnvalue_5) 0.0)
    (Transformation|SetActorRotation (Math|Rotator|MakeRotator (.roll _returnvalue_5) (.pitch _returnvalue_5) (- 1.8e+02 (* (.yaw _returnvalue_5) -1.0))))
    (else
      (Transformation|SetActorRotation (Math|Rotator|MakeRotator (.roll _returnvalue_5) (.pitch _returnvalue_5) (- 3.6e+02 (.yaw _returnvalue_5)))))))

(fn ConstructionScript)